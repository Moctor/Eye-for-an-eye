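; LevelMusic is a level actor that advances ambient music and the checkpoint as the player progresses through trigger boxes.
; On BeginPlay it caches BP_GameInstance, plays the first ambiance and stores Box0's location as the checkpoint.
; Box1 and Box2 overlaps from BP_PlayerInterface actors each fire once, saving that box's location and requesting the next ambiance through the GameInstance without stopping all sounds.
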(event OnComponentBeginOverlap(Box1)
  (params (OverlappedComponent :type Primitive%20Component%20Object%20Reference) (OtherActor :type Actor%20Object%20Reference) (OtherComp :type Primitive%20Component%20Object%20Reference) (OtherBodyIndex :type Integer) (bFromSweep :type Boolean) (SweepResult :type Hit%20Result%20Structure%20%28by%20ref%29))
  (if (Utilities|DoesObjectImplementInterface OtherActor "/Game/Blueprint/Player/BP_PlayerInterface.BP_PlayerInterface_C")
    (Utilities|FlowControl|DoOnce false
      (:Completed
        (Variables|/Game/Blueprint/BP_GameInstance.BP_GameInstance_C|SetCheckPointPosition (Variables|Default|GetGameInstance) (Transformation|GetWorldLocation (Variables|Default|GetBox1)))
        (Default|PlayLevelMusic01 (Variables|Default|GetGameInstance) "/Game/SFX/SoundCue/Ambiance2.Ambiance2" false)))))

(event OnComponentBeginOverlap(Box2)
  (params (OverlappedComponent :type Primitive%20Component%20Object%20Reference) (OtherActor :type Actor%20Object%20Reference) (OtherComp :type Primitive%20Component%20Object%20Reference) (OtherBodyIndex :type Integer) (bFromSweep :type Boolean) (SweepResult :type Hit%20Result%20Structure%20%28by%20ref%29))
  (if (Utilities|DoesObjectImplementInterface OtherActor "/Game/Blueprint/Player/BP_PlayerInterface.BP_PlayerInterface_C")
    (Utilities|FlowControl|DoOnce false
      (:Completed
        (Variables|/Game/Blueprint/BP_GameInstance.BP_GameInstance_C|SetCheckPointPosition (Variables|Default|GetGameInstance) (Transformation|GetWorldLocation (Variables|Default|GetBox2)))
        (Default|PlayLevelMusic01 (Variables|Default|GetGameInstance) "/Game/SFX/SoundCue/Ambiance3.Ambiance3" false)))))

(event EventBeginPlay
  (bind _asbp_game_instance (Utilities|Casting|CastToBP_GameInstance (Game|GetGameInstance)))
  (Variables|Default|SetGameInstance _asbp_game_instance)
  (Default|PlayLevelMusic01 (Variables|Default|GetGameInstance) "/Game/SFX/SoundCue/Ambiance1.Ambiance1" false)
  (Variables|/Game/Blueprint/BP_GameInstance.BP_GameInstance_C|SetCheckPointPosition (Variables|Default|GetGameInstance) (Transformation|GetWorldLocation (Variables|Default|GetBox0))))

(fn ConstructionScript)