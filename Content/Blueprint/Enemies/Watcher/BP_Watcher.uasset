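; Watcher enemy that sweeps a vision cone and sends a death message when it spots the player.
; A per-tick loop fans out line traces and scales instanced meshes to the hits, drawing a beam clipped by obstacles.
; Detection is separate: Tick checks the player's angle against the cone, then line-traces to them.
; Optional patrol lerps between angle limits, a timeline blinks the cone width, and the statue mesh can rotate along.
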(event Custom|Initialize
  ;[1 1 1] Initialize
  (Components|InstancedStaticMesh|ClearInstances (Variables|Default|GetInstancedStaticMesh))
  (for _index (range 0 (- (Variables|Public|GetMaxRay) 1))
    (Components|InstancedStaticMesh|AddInstance (Variables|Default|GetInstancedStaticMesh) (Math|Transform|MakeTransform "0, 0, 0" "0.000000,90.000000,0.000000") false))
  (CallFunction|SightTrace)
  (if (Variables|Public|GetHasPatrol)
    (Variables|Default|SetAimAngle (Variables|Public|GetMaxViewAngle))
    (CallFunction|InterpolationLoop)))

(event Custom|CheapInterpolationLoop
  (Variables|Default|SetAngleTimer (+ (Variables|Default|GetAngleTimer) (Utilities|Time|GetWorldDeltaSeconds))))

(event Custom|ChangeInstances
  (for _index (range (Variables|Default|GetNumberOfRay) (- (Variables|Public|GetMaxRay) 1))
    (Components|InstancedStaticMesh|UpdateInstanceTransform (Variables|Default|GetInstancedStaticMesh) _index (Math|Transform|MakeTransform "0, 0, 0" "0, 0, 0" "0.000000,0.000000,0.000000") false true true)))

(event Custom|InterpolationLoop
  ;[0.6266 1 0.6275] Interpolation Patrol
  (if (Variables|Default|GetIsEnable)
    (Variables|Default|SetAngleTimer (+ (Variables|Default|GetAngleTimer) (Utilities|Time|GetWorldDeltaSeconds)))
    (Variables|Default|SetCurrentAngle (Math|Float|Lerp (Math|Float|SelectFloat (Math|Float|SelectFloat (Variables|Public|GetMaxViewAngle) (Variables|Public|GetMinViewAngle) (Variables|Default|GetGoUp)) (Variables|Default|GetCurrentAngle) (Variables|Public|GetLinearInterpolation)) (Variables|Default|GetAimAngle) (/ (Variables|Default|GetAngleTimer) (Variables|Public|GetTimeSpeed))))
    (if (>= (/ (Variables|Default|GetAngleTimer) (Variables|Public|GetTimeSpeed)) 1.0)
      (Utilities|FlowControl|Delay (Variables|Public|GetWaitingTime))
      (bind _isa (Utilities|FlowControl|FlipFlop)
        (:A
          (Variables|Default|SetAimAngle (Variables|Public|GetMinViewAngle)))
        (:B
          (Variables|Default|SetAimAngle (Variables|Public|GetMaxViewAngle))))
      (Variables|Default|SetGoUp _isa)
      (Variables|Default|SetAngleTimer 0.0)
      (Utilities|FlowControl|DelayUntilNextTick)
      (CallFunction|InterpolationLoop)
      (else
        (Utilities|FlowControl|DelayUntilNextTick)
        (CallFunction|InterpolationLoop)))))

(event Custom|SightTrace
  (bind _returnvalue (Transformation|GetActorLocation))
  ;[1 1 1] Raycast + Mesh update
  (if (Variables|Default|GetIsEnable)
    (for _index (range 0 (- (Variables|Default|GetNumberOfRay) 1))
      (bind _output_get (Variables|Default|SetCurrentTrace _index))
      (bind (_outhit _returnvalue_2) (Collision|LineTraceForObjects _returnvalue (+ _returnvalue (* (Math|Vector|RotateVector (Math|Vector|GetUpVector (Transformation|GetActorRotation)) (Math|Rotator|MakeRotator (+ (- (* (Math|Conversions|ToFloat(Integer) _output_get) (/ (Variables|Public|GetDegreeAngleView) (Math|Conversions|ToFloat(Integer) (Variables|Default|GetNumberOfRay)))) (* (Variables|Public|GetDegreeAngleView) 0.5)) (Variables|Default|GetCurrentAngle)) 0.0 0.0)) (Variables|Public|GetMaxRange%28m%29) 1e+02)) (Variables|Default|GetObject%20Types) false 0 "None" true "(R=1.000000,G=0.000000,B=0.000000,A=1.000000)" "(R=0.000000,G=1.000000,B=0.000000,A=1.000000)" 0.1))
      (Components|InstancedStaticMesh|UpdateInstanceTransform (Variables|Default|GetInstancedStaticMesh) (Variables|Default|GetCurrentTrace) (Math|Transform|MakeTransform (Transformation|GetActorLocation) (Math|Rotator|CombineRotators (Transformation|GetWorldRotation (Variables|Default|GetInstancedStaticMesh)) (Math|Rotator|MakeRotator (+ (- (* (Math|Conversions|ToFloat(Integer) _output_get) (/ (Variables|Public|GetDegreeAngleView) (Math|Conversions|ToFloat(Integer) (Variables|Default|GetNumberOfRay)))) (* (Variables|Public|GetDegreeAngleView) 0.5)) (Variables|Default|GetCurrentAngle)) 0.0 0.0)) (Math|Vector|MakeVector (* (Math|Vector|VectorLength (- (Math|Vector|SelectVector (.location _outhit) (.traceend _outhit) _returnvalue_2) (.tracestart _outhit))) 0.01) (* (/ (Variables|Public|GetDegreeAngleView) (Math|Conversions|ToFloat(Integer) (Variables|Default|GetNumberOfRay))) (* (Math|Vector|VectorLength (- (Math|Vector|SelectVector (.location _outhit) (.traceend _outhit) _returnvalue_2) (.tracestart _outhit))) 0.01)) 25.0)) true true true))))

(event Custom|SphereDebug
  (bind _returnvalue (Transformation|GetActorRotation))
  (bind _instancedstaticmesh (Variables|Default|GetInstancedStaticMesh))
  (bind _maxrange_m_ (Variables|Public|GetMaxRange%28m%29))
  (bind _minviewangle (Variables|Public|GetMinViewAngle))
  (bind _maxrange_m__2 (Variables|Public|GetMaxRange%28m%29))
  (bind _maxviewangle (Variables|Public|GetMaxViewAngle))
  (bind _returnvalue_2 (Transformation|GetWorldLocation _instancedstaticmesh))
  (bind _returnvalue_3 (Math|Vector|GetUpVector _returnvalue))
  (bind _returnvalue_4 (* _maxrange_m_ 1e+02))
  (bind _returnvalue_5 (* _maxrange_m__2 1e+02))
  (bind _returnvalue_6 (Math|Vector|RotateVector _returnvalue_3 (Math|Rotator|MakeRotator _maxviewangle 0.0 0.0)))
  (bind _returnvalue_7 (Math|Vector|RotateVector _returnvalue_3 (Math|Rotator|MakeRotator _minviewangle 0.0 0.0)))
  (bind _returnvalue_8 (* _returnvalue_4 _returnvalue_6))
  (bind _returnvalue_9 (* _returnvalue_5 _returnvalue_7))
  (bind _returnvalue_10 (+ _returnvalue_2 _returnvalue_8))
  (bind _returnvalue_11 (+ _returnvalue_2 _returnvalue_9))
  ;[0.9157 1 0.383] Debug Editor
  (Rendering|Debug|DrawDebugCapsule _returnvalue_10 1.0 1e+01 "0, 0, 0" "(R=1.000000,G=0.000000,B=0.010493,A=1.000000)" 0.2 0.0)
  (Rendering|Debug|DrawDebugCapsule _returnvalue_11 1.0 1e+01 "0, 0, 0" "(R=1.000000,G=0.000000,B=0.010493,A=1.000000)" 0.2 0.0)
  (Transformation|SetWorldLocation (Variables|Default|GetMaxSphere) _returnvalue_10 false true)
  (Transformation|SetWorldLocation (Variables|Default|GetMinSphere) _returnvalue_11 false true))

(event Custom|OptiLoop
  (Variables|Default|SetNumberOfRay (Variables|Public|GetMaxRay))
  (Utilities|FlowControl|DelayUntilNextTick)
  (CallFunction|ChangeInstances)
  (CallFunction|OptiLoop)
  (CallFunction|SightTrace))

(event EventBeginPlay
  ;[1 1 1] Start
  (CallFunction|OptiLoop)
  (CallFunction|Initialize)
  (Components|DestroyComponent (Variables|Default|GetMaxSphere))
  (Components|DestroyComponent (Variables|Default|GetMinSphere))
  (Variables|Default|SetTrackRotation (- (* (* (Variables|Public|GetMaxRay) 0.5) (/ (Variables|Public|GetDegreeAngleView) (Math|Conversions|ToFloat(Integer) (Variables|Default|GetNumberOfRay)))) (+ (.z (Math|Vector|GetUpVector (Transformation|GetWorldRotation (Variables|Default|GetInstancedStaticMesh)))) (* (Variables|Public|GetDegreeAngleView) 0.5))))
  (Variables|Default|SetPlayerRef (Game|GetPlayerController 0))
  (if (Variables|Default|GetIsBlinking)
    (bind _field_of_view (Timeline|Timeline Play)
      (:Update
        (Variables|Public|SetDegreeAngleView _field_of_view))
      (:Finished
        (Utilities|FlowControl|Delay 0.1)
        (Timeline|Timeline PlayFromStart)))))

(event EventTick
  (params (DeltaSeconds :type Float%20%28single-precision%29))
  (bind _returnvalue (Transformation|GetActorLocation))
  (bind _statuemesh (Variables|Default|GetStatueMesh))
  (bind _degreeangleview (Variables|Public|GetDegreeAngleView))
  (bind _defaultsceneroot (Variables|Default|GetDefaultSceneRoot))
  (bind _statuemesh_2 (Variables|Default|GetStatueMesh))
  (bind _instancedstaticmesh (Variables|Default|GetInstancedStaticMesh))
  (bind _playerref (Variables|Default|GetPlayerRef))
  (bind _playerref_2 (Variables|Default|GetPlayerRef))
  (bind _returnvalue_2 (Transformation|GetWorldLocation _defaultsceneroot))
  (bind _returnvalue_3 (Transformation|GetWorldLocation _statuemesh))
  (bind _returnvalue_4 (Transformation|GetWorldRotation _statuemesh_2))
  (bind _returnvalue_5 (Transformation|GetActorLocation _playerref_2))
  (bind _returnvalue_6 (Transformation|GetWorldRotation _instancedstaticmesh))
  (bind _returnvalue_7 (* _degreeangleview 0.5))
  (bind _returnvalue_8 (Math|Vector|GetForwardVector _returnvalue_6))
  (bind _returnvalue_9 (- _returnvalue_5 _returnvalue))
  (bind _returnvalue_10 (- _returnvalue_2 _returnvalue_3))
  (bind (_x _y _z) (Math|Vector|BreakVector _returnvalue_9))
  (bind (_x_2 _y_2 _z_2) (Math|Vector|BreakVector _returnvalue_8))
  (bind _returnvalue_11 (Math|Vector|MakeVector 0.0 _y _z))
  (bind _returnvalue_12 (Math|Vector|MakeVector 0.0 _y_2 _z_2))
  (bind _returnvalue_13 (Math|Vector|Normalize _returnvalue_12))
  (bind _returnvalue_14 (Math|Vector|Normalize _returnvalue_11))
  (bind _returnvalue_15 (Math|Vector|DotProduct _returnvalue_13 _returnvalue_14))
  (bind _returnvalue_16 (- 1.0 _returnvalue_15))
  (bind _returnvalue_17 (* _returnvalue_16 1.8e+02))
  (Utilities|FlowControl|Sequence
    (:then_0
      (Utilities|IsValid _playerref
        (:Is%20Valid
          (if (and (< _returnvalue_17 (+ (Variables|Default|GetCurrentAngle) _returnvalue_7)) (> _returnvalue_17 (- (Variables|Default|GetCurrentAngle) _returnvalue_7)))
            (bind (_outhit _returnvalue_18) (Collision|LineTraceForObjects (Transformation|GetActorLocation) (Transformation|GetActorLocation _playerref) (Variables|Default|GetObject%20Types) false 0 "None" true "(R=1.000000,G=0.000000,B=0.000000,A=1.000000)" "(R=0.000000,G=1.000000,B=0.000000,A=1.000000)" 0.1))
            (if _returnvalue_18
              (if (Utilities|DoesObjectImplementInterface (.hitactor _outhit) "/Game/Blueprint/Player/BP_PlayerInterface.BP_PlayerInterface_C")
                (Class|BPPlayerInterface|Death(Message) (.hitactor _outhit)))
              (else
                (if true :!label _label
                  (Variables|Default|SetDieCounter (- (Variables|Default|GetDieCounter) (Utilities|Time|GetWorldDeltaSeconds))))))
            (else
              (goto _label))))))
    (:then_1
      (if (Variables|Default|GetIsRotating)
        (Transformation|AddWorldOffset _statuemesh _returnvalue_10 true true)
        (Transformation|SetWorldRotation _statuemesh_2 (Math|Rotator|MakeRotator (.roll _returnvalue_4) (- (Variables|Default|GetTrackRotation) (Variables|Default|GetCurrentAngle)) (.yaw _returnvalue_4)) false false)
        (Transformation|AddWorldOffset _statuemesh (* _returnvalue_10 -1.0) true true)))))

(fn ConstructionScript
  (CallFunction|Initialize)
  (CallFunction|SphereDebug))