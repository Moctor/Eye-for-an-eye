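; Spike trap enemy Blueprint whose spikes periodically rise and retract, killing what enters its collision box while they are up.
; On BeginPlay a looping timer fires the spike cycle, which eases the mesh up with a 2D sound, waits, then lowers it.
; A CanKill flag is set during the rise and cleared after retraction; overlap begin then sends a death message to interface-implementing actors.
; Only new overlaps trigger a kill.
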(event OnComponentBeginOverlap(BoxColision)
  (params (OverlappedComponent :type Primitive%20Component%20Object%20Reference) (OtherActor :type Actor%20Object%20Reference) (OtherComp :type Primitive%20Component%20Object%20Reference) (OtherBodyIndex :type Integer) (bFromSweep :type Boolean) (SweepResult :type Hit%20Result%20Structure%20%28by%20ref%29))
  (if (and (Utilities|DoesObjectImplementInterface OtherActor (Variables|Default|GetInterface)) (Variables|Default|GetCanKill?))
    (Class|BPPlayerInterface|Death(Message) OtherActor)))

(event OnComponentEndOverlap(BoxColision)
  (params (OverlappedComponent :type Primitive%20Component%20Object%20Reference) (OtherActor :type Actor%20Object%20Reference) (OtherComp :type Primitive%20Component%20Object%20Reference) (OtherBodyIndex :type Integer))
  (if (Utilities|DoesObjectImplementInterface OtherActor (Variables|Default|GetInterface))
    _))

(event Custom|ActivationSpyke
  ;[1 1 1] Fais spawn Des spykes tout les x temps
  (bind _returnvalue (Utilities|Time|SetTimerbyEvent (delegate Custom|SpawnSpkye) (Variables|Default|GetTimerSpkye) true))
  (Variables|Default|SetSpykeTimer _returnvalue))

(event Custom|SpawnSpkye
  ;[1 1 1] Fais spawn Des spykes tout les x temps
  (Variables|Default|SetCanKill? true)
  (Components|MoveComponentTo (Variables|Default|GetSpikeTrap) (Math|Vector|MakeVector 0.0 0.0 (Variables|Default|GetSpikeHeight)) "0, 0, 0" true true (* (Variables|Default|GetDelaySpyke) 0.5) false)
  (bind _returnvalue (Audio|CreateSound2D "/Game/SFX/SoundCue/Piege.Piege" 0.75 1.0 0.0 0))
  (Audio|Components|Audio|Play _returnvalue 0.0)
  (Utilities|FlowControl|Delay (* (Variables|Default|GetDelaySpyke) 0.5))
  (Components|MoveComponentTo (Variables|Default|GetSpikeTrap) (Math|Vector|MakeVector 0.0 0.0 -5e+01) "0, 0, 0" true true (* (Variables|Default|GetDelaySpyke) 0.5) false)
  (Variables|Default|SetCanKill? false))

(event EventBeginPlay
  (|CallParentFunction)
  (CallFunction|ActivationSpyke))

(event Collision|EventActorBeginOverlap
  (params (OtherActor :type Actor%20Object%20Reference))
  (|CallParentFunction OtherActor) ; This node is disabled and will not be called.\nDrag off pins to build functionality.
)

(event EventTick
  (params (DeltaSeconds :type Float%20%28single-precision%29))
  (|CallParentFunction DeltaSeconds) ; This node is disabled and will not be called.\nDrag off pins to build functionality.
)

(fn ConstructionScript
  (|CallParentFunction))