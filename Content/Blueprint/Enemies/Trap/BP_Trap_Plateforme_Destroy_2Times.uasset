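; Trap platform that is destroyed the second time a player steps on it.
; A Box begin-overlap accepts only actors implementing BP_PlayerInterface and feeds a FlipFlop.
; The first valid overlap swaps the Mesh material to a second platform material, and the next destroys the actor.
; BeginPlay, Tick and construction only call the parent versions.
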(event OnComponentBeginOverlap(Box)
  (params (OverlappedComponent :type Primitive%20Component%20Object%20Reference) (OtherActor :type Actor%20Object%20Reference) (OtherComp :type Primitive%20Component%20Object%20Reference) (OtherBodyIndex :type Integer) (bFromSweep :type Boolean) (SweepResult :type Hit%20Result%20Structure%20%28by%20ref%29))
  ;[0.7031 0.0122 0.01453] Begin overlap Plateforme
  ;;[0.06771 0.06771 0.06771] Check si il a l'interface
  (if (Utilities|DoesObjectImplementInterface OtherActor "/Game/Blueprint/Player/BP_PlayerInterface.BP_PlayerInterface_C")
    (Utilities|FlowControl|FlipFlop
      (:A
        (Rendering|Material|SetMaterial (Variables|Default|GetMesh) 0 "/Game/Materials/Environment/MI_Platform_Medium_2.MI_Platform_Medium_2"))
      (:B
        ;;[0.06771 0.06771 0.06771] Detruit la plateforme
        (Actor|DestroyActor)))))

(event EventBeginPlay
  (|CallParentFunction))

(event Collision|EventActorBeginOverlap
  (params (OtherActor :type Actor%20Object%20Reference))
  (|CallParentFunction OtherActor) ; This node is disabled and will not be called.\nDrag off pins to build functionality.
)

(event EventTick
  (params (DeltaSeconds :type Float%20%28single-precision%29))
  (|CallParentFunction DeltaSeconds))

(fn ConstructionScript
  (|CallParentFunction))