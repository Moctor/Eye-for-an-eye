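; Spike trap that rises when a player enters its call volume and kills on contact while active.
; CallSpike overlaps drive MoveComponentTo on SpikeTrap, raising it quickly on entry and lowering it over DisableTime on exit, each with a sound.
; KillTrigger sends DeathMessage to actors implementing BP_PlayerInterface only while IsActive is set.
; IsActive clears at three-quarters of DisableTime after exit, before the spikes fully retract.
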(event OnComponentBeginOverlap(CallSpike)
  (params (OverlappedComponent :type Primitive%20Component%20Object%20Reference) (OtherActor :type Actor%20Object%20Reference) (OtherComp :type Primitive%20Component%20Object%20Reference) (OtherBodyIndex :type Integer) (bFromSweep :type Boolean) (SweepResult :type Hit%20Result%20Structure%20%28by%20ref%29))
  ;[1 1 1] Move Trap
  (if (Utilities|DoesObjectImplementInterface OtherActor "/Game/Blueprint/Player/BP_PlayerInterface.BP_PlayerInterface_C")
    (Variables|Default|SetIsActive true)
    (Components|MoveComponentTo (Variables|Default|GetSpikeTrap) (Math|Vector|MakeVector 0.0 0.0 -4.5) "0, 0, 0" true false 0.15 false)
    (bind _returnvalue (Audio|CreateSound2D "/Game/SFX/SoundCue/Piege.Piege" 0.75 1.0 0.0 0))
    (Audio|Components|Audio|Play _returnvalue 0.0)))

(event OnComponentEndOverlap(CallSpike)
  (params (OverlappedComponent :type Primitive%20Component%20Object%20Reference) (OtherActor :type Actor%20Object%20Reference) (OtherComp :type Primitive%20Component%20Object%20Reference) (OtherBodyIndex :type Integer))
  ;[1 1 1] Move Trap
  (if (Utilities|DoesObjectImplementInterface OtherActor "/Game/Blueprint/Player/BP_PlayerInterface.BP_PlayerInterface_C")
    (Utilities|FlowControl|Sequence
      (:then_0
        (Components|MoveComponentTo (Variables|Default|GetSpikeTrap) (Math|Vector|MakeVector 0.0 0.0 -5e+01) "0, 0, 0" true true (Variables|Default|GetDisableTime) false)
        (bind _returnvalue (Audio|CreateSound2D "/Game/SFX/SoundCue/Piege.Piege" 0.75 -1.0 0.0 0))
        (Audio|Components|Audio|Play _returnvalue 0.0))
      (:then_1
        (Utilities|FlowControl|Delay (* (Variables|Default|GetDisableTime) 0.75))
        (Variables|Default|SetIsActive false)))))

(event OnComponentBeginOverlap(KillTrigger)
  (params (OverlappedComponent :type Primitive%20Component%20Object%20Reference) (OtherActor :type Actor%20Object%20Reference) (OtherComp :type Primitive%20Component%20Object%20Reference) (OtherBodyIndex :type Integer) (bFromSweep :type Boolean) (SweepResult :type Hit%20Result%20Structure%20%28by%20ref%29))
  (if (and (Utilities|DoesObjectImplementInterface OtherActor "/Game/Blueprint/Player/BP_PlayerInterface.BP_PlayerInterface_C") (Variables|Default|GetIsActive))
    (Class|BPPlayerInterface|Death(Message) OtherActor)))

(event EventBeginPlay
  (|CallParentFunction) ; This node is disabled and will not be called.\nDrag off pins to build functionality.
)

(event Collision|EventActorBeginOverlap
  (params (OtherActor :type Actor%20Object%20Reference))
  (|CallParentFunction OtherActor) ; This node is disabled and will not be called.\nDrag off pins to build functionality.
)

(event EventTick
  (params (DeltaSeconds :type Float%20%28single-precision%29))
  (|CallParentFunction DeltaSeconds) ; This node is disabled and will not be called.\nDrag off pins to build functionality.
)

(fn ConstructionScript
  (|CallParentFunction))