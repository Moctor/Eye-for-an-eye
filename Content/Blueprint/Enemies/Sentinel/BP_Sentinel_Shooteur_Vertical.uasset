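; Vertical variant of the shooter Sentinel enemy that moves its mesh along the Z axis.
; BeginPlay stores the mesh's world start location and sets DistanceMid as the target height.
; Each Tick advances a timer scaled by Vitesse, whose fractional part samples CurveTranslation to lerp Z between start and target, repeating every cycle.
; The target is used as a world Z rather than an offset, and this graph contains no shooting logic.
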(event EventBeginPlay
  ;[0.2127 0.8633 1] BeginPlay
  (|CallParentFunction)
  ;;[0.1372 0.1372 0.1372] Stocke sa position de dépard
  (Variables|Default|SetStartLocation (Transformation|GetWorldLocation (Variables|Character|GetMesh)))
  ;;[0.1094 0.1094 0.1094] Set son déplacement à faire en premier
  (Variables|Default|SetCurrentTarget (Variables|Default|GetDistanceMid)))

(event Collision|EventActorBeginOverlap
  (params (OtherActor :type Actor%20Object%20Reference))
  (|CallParentFunction OtherActor) ; This node is disabled and will not be called.\nDrag off pins to build functionality.
)

(event EventTick
  (params (DeltaSeconds :type Float%20%28single-precision%29))
  (bind _startlocation (Variables|Default|GetStartLocation))
  (bind (_x _y _z) (Class|KismetMathLibrary|BreakVector3f _startlocation))
  ;[0.5851 0.4999 0.08634] EvenTick
  (|CallParentFunction 0.0)
  ;;[0.1094 0.1094 0.1094] Set un Timer pour le déplacement en fonction de sa vitesse
  (Variables|Default|SetTimer (+ (Variables|Default|GetTimer) (* DeltaSeconds (Variables|Default|GetVitesse))))
  ;;[0.1094 0.1094 0.1094] Effectue son déplacement
  (Transformation|SetWorldLocation (Variables|Character|GetMesh) (Math|Vector|MakeVector _x _y (Math|Float|Lerp _z (Variables|Default|GetCurrentTarget) (Math|Curves|GetFloatValue (Variables|Default|GetCurveTranslation) (Math|Float|Fraction (Variables|Default|GetTimer))))) false false))

(fn ConstructionScript
  (|CallParentFunction))