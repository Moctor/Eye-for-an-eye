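; Sentinel enemy variant that endlessly moves its mesh around a rectangular loop in its relative Y-Z plane.
; BeginPlay records the mesh's start position and derives four leg targets from negative and positive distance values.
; Tick calls the parent, advances a speed-scaled timer, and lerps one axis per leg through a translation curve.
; Boolean flags act as a four-state cycle, resetting the timer and start point after each leg.
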(event EventBeginPlay
  (Variables|Default|SetStarterPoint (Variables|/Script/Engine.SceneComponent|GetRelativeLocation (Variables|Character|GetMesh)))
  (Variables|Default|SetFirstLocation (Variables|Default|GetDistanceNeg))
  (Variables|Default|SetSecondLocation (Variables|Default|GetDistanceNeg))
  (Variables|Default|SetThirdLocation (Variables|Default|GetDistancePos))
  (Variables|Default|SetFourthLocation (Variables|Default|GetDistancePos))
  (Variables|Default|SetFirstLocation? true))

(event Collision|EventActorBeginOverlap
  (params (OtherActor :type Actor%20Object%20Reference))
  (|CallParentFunction OtherActor) ; This node is disabled and will not be called.\nDrag off pins to build functionality.
)

(event EventTick
  (params (DeltaSeconds :type Float%20%28single-precision%29))
  (|CallParentFunction DeltaSeconds)
  ;[0.1094 0.1094 0.1094] Set un Timer pour le déplacement en fonction de sa vitesse
  (Variables|Default|SetTimer (+ (Variables|Default|GetTimer) (* DeltaSeconds (Variables|Default|GetVitesse))))
  (Utilities|FlowControl|Sequence
    (:then_0
      (if (Variables|Default|GetFirstLocation?)
        ;[0.1094 0.1094 0.1094] Effectue son déplacement
        (Transformation|SetRelativeLocation (Variables|Character|GetMesh) (Math|Vector|MakeVector (.X (Class|KismetMathLibrary|BreakVector3f (Variables|Default|GetStarterPoint))) (Math|Float|Lerp (.Y (Class|KismetMathLibrary|BreakVector3f (Variables|Default|GetStarterPoint))) (Variables|Default|GetFirstLocation) (Math|Curves|GetFloatValue (Variables|Default|GetCurveTranslation) (Variables|Default|GetTimer))) (.Z (Class|KismetMathLibrary|BreakVector3f (Variables|Default|GetStarterPoint)))) false false)
        (if (>= (Variables|Default|GetTimer) 1.0)
          (Variables|Default|SetStarterPoint (Variables|/Script/Engine.SceneComponent|GetRelativeLocation (Variables|Character|GetMesh)))
          (Variables|Default|SetTimer 0.0)
          (Variables|Default|SetSecondLocation? true)
          (Variables|Default|SetFirstLocation? false))))
    (:then_1
      (if (Variables|Default|GetSecondLocation?)
        ;[0.1094 0.1094 0.1094] Effectue son déplacement
        (Transformation|SetRelativeLocation (Variables|Character|GetMesh) (Math|Vector|MakeVector (.X (Class|KismetMathLibrary|BreakVector3f (Variables|Default|GetStarterPoint))) (.Y (Class|KismetMathLibrary|BreakVector3f (Variables|Default|GetStarterPoint))) (Math|Float|Lerp (.Z (Class|KismetMathLibrary|BreakVector3f (Variables|Default|GetStarterPoint))) (Variables|Default|GetSecondLocation) (Math|Curves|GetFloatValue (Variables|Default|GetCurveTranslation) (Variables|Default|GetTimer)))) false false)
        (if (>= (Variables|Default|GetTimer) 1.0)
          (Variables|Default|SetStarterPoint (Variables|/Script/Engine.SceneComponent|GetRelativeLocation (Variables|Character|GetMesh)))
          (Variables|Default|SetTimer 0.0)
          (Variables|Default|SetThirdLocation? true)
          (Variables|Default|SetSecondLocation? false))))
    (:then_2
      (if (Variables|Default|GetThirdLocation?)
        ;[0.1094 0.1094 0.1094] Effectue son déplacement
        (Transformation|SetRelativeLocation (Variables|Character|GetMesh) (Math|Vector|MakeVector (.X (Class|KismetMathLibrary|BreakVector3f (Variables|Default|GetStarterPoint))) (Math|Float|Lerp (.Y (Class|KismetMathLibrary|BreakVector3f (Variables|Default|GetStarterPoint))) (Variables|Default|GetThirdLocation) (Math|Curves|GetFloatValue (Variables|Default|GetCurveTranslation) (Variables|Default|GetTimer))) (.Z (Class|KismetMathLibrary|BreakVector3f (Variables|Default|GetStarterPoint)))) false false)
        (if (>= (Variables|Default|GetTimer) 1.0)
          (Variables|Default|SetStarterPoint (Variables|/Script/Engine.SceneComponent|GetRelativeLocation (Variables|Character|GetMesh)))
          (Variables|Default|SetTimer 0.0)
          (Variables|Default|SetFourthLocation? true)
          (Variables|Default|SetThirdLocation? false))))
    (:then_3
      (if (Variables|Default|GetFourthLocation?)
        ;[0.1094 0.1094 0.1094] Effectue son déplacement
        (Transformation|SetRelativeLocation (Variables|Character|GetMesh) (Math|Vector|MakeVector (.X (Class|KismetMathLibrary|BreakVector3f (Variables|Default|GetStarterPoint))) (.Y (Class|KismetMathLibrary|BreakVector3f (Variables|Default|GetStarterPoint))) (Math|Float|Lerp (.Z (Class|KismetMathLibrary|BreakVector3f (Variables|Default|GetStarterPoint))) (Variables|Default|GetFourthLocation) (Math|Curves|GetFloatValue (Variables|Default|GetCurveTranslation) (Variables|Default|GetTimer)))) false false)
        (if (>= (Variables|Default|GetTimer) 1.0)
          (Variables|Default|SetStarterPoint (Variables|/Script/Engine.SceneComponent|GetRelativeLocation (Variables|Character|GetMesh)))
          (Variables|Default|SetTimer 0.0)
          (Variables|Default|SetFirstLocation? true)
          (Variables|Default|SetFourthLocation? false))))))

(fn ConstructionScript
  (|CallParentFunction))