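; BP_Sentinel_Horizontal is a Sentinel enemy variant that slides its mesh horizontally along the world Y axis.
; BeginPlay stores the mesh's starting location and takes MidDistance as the target Y coordinate.
; Each Tick advances a timer scaled by Vitesse (speed), whose fractional part samples CurveTranslation to lerp between start and target Y, producing looping, curve-shaped movement with fixed X and Z.
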(event EventBeginPlay
  (|CallParentFunction)
  (Variables|Default|SetStartLocation (Transformation|GetWorldLocation (Variables|Character|GetMesh)))
  (Variables|Default|SetcurrentTargetLocation (Variables|Default|GetMidDistance)))

(event Collision|EventActorBeginOverlap
  (params (OtherActor :type Actor%20Object%20Reference))
  (|CallParentFunction OtherActor) ; This node is disabled and will not be called.\nDrag off pins to build functionality.
)

(event EventTick
  (params (DeltaSeconds :type Float%20%28single-precision%29))
  (bind _startlocation (Variables|Default|GetStartLocation))
  (bind (_x _y _z) (Class|KismetMathLibrary|BreakVector3f _startlocation))
  (|CallParentFunction DeltaSeconds)
  ;[0.1094 0.1094 0.1094] Set un Timer pour le déplacement en fonction de sa vitesse
  (Variables|Default|SetTimer (+ (Variables|Default|GetTimer) (* DeltaSeconds (Variables|Default|GetVitesse))))
  ;[0.1094 0.1094 0.1094] Effectue son déplacement
  (Transformation|SetWorldLocation (Variables|Character|GetMesh) (Math|Vector|MakeVector _x (Math|Float|Lerp _y (Variables|Default|GetcurrentTargetLocation) (Math|Curves|GetFloatValue (Variables|Default|GetCurveTranslation) (Math|Float|Fraction (Variables|Default|GetTimer)))) _z) false false))

(fn ConstructionScript
  (|CallParentFunction))