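; Static shooter Sentinel enemy that animates its mesh with a looping roll rotation; no firing logic appears here.
; BeginPlay stores the mesh's starting world rotation and sets MidRotationDistance as the target roll.
; Tick advances a timer scaled by Vitesse and feeds its fractional part into CurveTranslation.
; The curve value drives a Lerp from starting roll to target, keeping pitch and yaw at their initial values.
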(event EventBeginPlay
  (|CallParentFunction)
  (Variables|Default|SetStartRotation (Transformation|GetWorldRotation (Variables|Character|GetMesh)))
  (Variables|Default|SetCurrentTargetRotation (Variables|Default|GetMidRotationDistance)))

(event Collision|EventActorBeginOverlap
  (params (OtherActor :type Actor%20Object%20Reference))
  (|CallParentFunction OtherActor) ; This node is disabled and will not be called.\nDrag off pins to build functionality.
)

(event EventTick
  (params (DeltaSeconds :type Float%20%28single-precision%29))
  (bind _startrotation (Variables|Default|GetStartRotation))
  (bind _returnvalue (Math|Rotator|GetRotationXVector _startrotation))
  (|CallParentFunction DeltaSeconds)
  ;[0.1094 0.1094 0.1094] Set un Timer pour le déplacement en fonction de sa vitesse
  (Variables|Default|SetTimer (+ (Variables|Default|GetTimer) (* DeltaSeconds (Variables|Default|GetVitesse))))
  ;[0.1094 0.1094 0.1094] Effectue son déplacement
  (Transformation|SetWorldRotation (Variables|Character|GetMesh) (Math|Rotator|MakeRotator (Math|Float|Lerp (.x _returnvalue) (Variables|Default|GetCurrentTargetRotation) (Math|Curves|GetFloatValue (Variables|Default|GetCurveTranslation) (Math|Float|Fraction (Variables|Default|GetTimer)))) (.y _returnvalue) (.z _returnvalue)) false false))

(fn ConstructionScript
  (|CallParentFunction))