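; Sentinel shooter enemy Blueprint that fires fire spike projectiles continuously from the moment play begins.
; BeginPlay starts a looping timer whose interval is the inverse of ShootSeconds plus a random offset, rolled once so each instance keeps its own fire rate.
; Each timer tick spawns a BP_Projectiles_Sentinelle_FireSpyke at the Arrow component's transform and plays a non-spatialized wind projectile sound, with no targeting logic.
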(event Custom|Shooting
  ;[0.07118 0.07118 0.07118] Tire un projectile
  (Utilities|Time|SetTimerbyEvent (delegate Custom|Shoot) (/ 1.0 (+ (Variables|Default|GetShoot/Seconds) (Math|Random|RandomFloatinRange 0.0 5.0))) true))

(event Custom|Shoot
  ;[0.07118 0.07118 0.07118] Tire un projectile
  (Game|SpawnActorfromClass "/Game/Blueprint/Projectiles/BP_Projectiles_Sentinelle_FireSpyke.BP_Projectiles_Sentinelle_FireSpyke_C" (Transformation|GetWorldTransform (Variables|Default|GetArrow)) "Undefined" 0 0)
  (Audio|PlaySound2D "/Game/SFX/SoundCue/SFX_Wind_Projectiles.SFX_Wind_Projectiles" 1.0 1.0 0.0 0 0))

(event EventBeginPlay
  (|CallParentFunction)
  ;[0.0816 0.0816 0.0816] Tire
  (CallFunction|Shooting))

(event Collision|EventActorBeginOverlap
  (params (OtherActor :type Actor%20Object%20Reference))
  (|CallParentFunction OtherActor) ; This node is disabled and will not be called.\nDrag off pins to build functionality.
)

(event EventTick
  (params (DeltaSeconds :type Float%20%28single-precision%29))
  (|CallParentFunction DeltaSeconds) ; This node is disabled and will not be called.\nDrag off pins to build functionality.
)

(fn ConstructionScript
  (|CallParentFunction))