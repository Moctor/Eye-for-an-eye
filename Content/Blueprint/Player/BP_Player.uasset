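; Player Blueprint for a physics-driven character moving in the Y-Z plane, with jump, dash, checkpoint respawn and win screen.
; Input drives SkeletalMesh velocity, forces and impulses, using curves for acceleration and jump, while dash briefly disables gravity.
; Tick handles vertical camera follow, ground traces that re-arm jump and dash, fake gravity, and impact shakes from velocity changes.
; A helmet absorbs one death; otherwise a red material fade precedes respawn at the GameInstance checkpoint.
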(event Custom|ResetJump
  ;[1 1 1] Jump Functions
  (Variables|Default|SetIsJumping false)
  (Variables|Default|SetJumpTime 0.0)
  (Variables|Default|SetCanJump false))

(event Custom|ResetDash
  (bind _dashstrength (Variables|Default|GetDashStrength))
  (bind _skeletalmesh (Variables|Default|GetSkeletalMesh))
  (bind _skeletalmesh_2 (Variables|Default|GetSkeletalMesh))
  (bind _verticalsign (Variables|Default|GetVerticalSign))
  (bind _returnvalue (Transformation|GetComponentVelocity _skeletalmesh_2))
  (bind _returnvalue_2 (Transformation|GetWorldLocation _skeletalmesh))
  (bind _returnvalue_3 (< _verticalsign 0.0))
  (bind _returnvalue_4 (< (.z _returnvalue) 0.0))
  (bind _returnvalue_5 (and _returnvalue_4 _returnvalue_3))
  ;[1 1 1] Dash Function
  (Physics|SetEnableGravity (Variables|Default|GetSkeletalMesh) true)
  (Variables|Default|SetIsDashing false)
  (Utilities|FlowControl|Delay 0.5)
  (Utilities|FlowControl|Gate false) ; enters at Open
)

(event Custom|DeathVFX
  (Niagara|SpawnSystematLocation 0 (Transformation|GetWorldLocation (Variables|Default|GetSkeletalMesh)) "0, 0, 0" "0.500000,0.500000,0.500000")
  (bind _output_get (Variables|Default|SetAlphaVFX (+ (Variables|Default|GetAlphaVFX) 0.5) :!label _label))
  (Rendering|Material|SetScalarParameterValue (Variables|Default|GetDynamicMaterialInstance) "RedTransition" (Class|KismetMathLibrary|FInterpEaseinOut 0.0 1.0 _output_get 0.0) :!class /Script/Engine.MaterialInstanceDynamic)
  (if (< _output_get 1.0)
    (Utilities|FlowControl|Delay 0.1)
    (goto _label)))

(event Custom|ResetPlayer
  (Transformation|SetWorldLocation (Variables|Default|GetSkeletalMesh) (Variables|/Game/Blueprint/BP_GameInstance.BP_GameInstance_C|GetCheckPointPosition (Variables|Default|GetGameInstance)) false true)
  (Input|EnableInput (Game|GetPlayerController 0))
  (Variables|Default|SetAlphaVFX 0.0)
  (Rendering|Material|SetScalarParameterValue (Variables|Default|GetDynamicMaterialInstance) "RedTransition" 0.0 :!class /Script/Engine.MaterialInstanceDynamic)
  (Variables|Default|SetImmune false))

(event EventWinGame
  ;[1 1 1] WinGame
  (Input|DisableInput (Game|GetPlayerController 0))
  (bind _returnvalue (UserInterface|CreateWidget "/Game/Widget/Menu/WBP_WinMenu.WBP_WinMenu_C"))
  (UserInterface|Viewport|AddtoViewport _returnvalue 0)
  (Utilities|FlowControl|Delay 3.0)
  (Game|OpenLevel(byObjectReference) "/Game/Level/MenuTest.MenuTest"))

(event EventEarnAHelmet
  (bind _helmet (Variables|Default|GetHelmet))
  (Rendering|SetVisibility (Variables|Default|GetHelmet) true false)
  (Variables|Default|SetHasHelmet true)
  (bind (_direction _scale _rotation _positionoffset) (Timeline|Le%20chapeau PlayFromStart)
    (:Update
      (Transformation|SetRelativeScale3D _helmet (Math|Conversions|ToVector(Float) _scale))
      (Transformation|SetRelativeRotation _helmet (Math|Rotator|MakeRotator 9e+01 _rotation 1.8e+02) false false)
      (Transformation|SetRelativeLocation _helmet (Math|Vector|MakeVector 0.0 3.647981 (* _positionoffset 25.0)) false false))
    (:Finished
      (Niagara|SpawnSystematLocation "/Game/VFX/Helmet/SparkleHelmet.SparkleHelmet" (+ (Transformation|GetWorldLocation (Variables|Default|GetSkeletalMesh)) "0.000000,0.000000,50.834964") "0, 0, 0" "1.000000,1.000000,1.000000" true true "None" false))))

(event EventTick
  (params (DeltaSeconds :type Float%20%28single-precision%29))
  (bind _skeletalmesh (Variables|Default|GetSkeletalMesh))
  (bind _skeletalmesh_2 (Variables|Default|GetSkeletalMesh))
  (bind _springarm (Variables|Default|GetSpringArm))
  (bind _decaldegeu (Variables|Default|GetDecalDegeu))
  (bind _returnvalue (Transformation|GetWorldLocation _springarm))
  (bind _returnvalue_2 (Transformation|GetWorldLocation _skeletalmesh))
  (bind _returnvalue_3 (Transformation|GetComponentVelocity _skeletalmesh_2))
  (Utilities|FlowControl|Sequence
    (:then_0
      ;[1 1 1] Camera Follow
      (Transformation|SetWorldLocation _springarm (Math|Vector|MakeVector (.x _returnvalue) (.y _returnvalue) (Math|Float|Clamp(Float) (+ (.z _returnvalue) (- (- (.z (Transformation|GetWorldLocation (Variables|Default|GetSkeletalMesh))) (Variables|Default|GetCameraVerticalOffset)) (.z _returnvalue))) -2.03e+04 0.0)) false false))
    (:then_1
      ;[1 1 1] Check Ground distance
      (if (not (or (Variables|Default|GetIsDashing) (Variables|Default|GetIsJumping)))
        (bind _returnvalue_4 (Collision|LineTraceByChannel _returnvalue_2 (- _returnvalue_2 (Math|Vector|MakeVector 0.0 0.0 (Variables|Default|GetCheckGroundDistance))) "TraceTypeQuery1" false 0 "None" true "(R=1.000000,G=0.000000,B=0.000000,A=1.000000)" "(R=0.000000,G=1.000000,B=0.000000,A=1.000000)" 0.1 :!label _label))
        (if _returnvalue_4
          (Variables|Default|SetCanJump true)
          (Variables|Default|SetCanDash true)
          (goto _label_2 Open)
          (else
            (Utilities|FlowControl|Gate false :!label _label_2
              (:Exit
                (Utilities|FlowControl|Sequence
                  (:then_0
                    (Utilities|FlowControl|Delay (Variables|Default|GetJumpCooldown))
                    (Variables|Default|SetCanJump false)
                    (goto _label))
                  (:then_1
                    (goto _label_2 Close)))))))))
    (:then_2
      ;[1 1 1] Fake Gravity
      (Physics|AddForce (Variables|Default|GetSkeletalMesh) (Math|Vector|MakeVector 0.0 0.0 (Variables|Default|GetFakeGravity)) "None" false))
    (:then_3
      ;[0 0 0] Jump Time
      (if (Variables|Default|GetIsJumping)
        (Variables|Default|SetJumpTime (Math|Float|Clamp(Float) (+ (Variables|Default|GetJumpTime) (* DeltaSeconds (Variables|Default|GetJumpTimeSpeed)))))
        (Physics|AddForce (Variables|Default|GetSkeletalMesh) (Math|Vector|MakeVector 0.0 0.0 (* (Math|Curves|GetFloatValue (Variables|Default|GetJumpCurve) (Variables|Default|GetJumpTime)) (Variables|Default|GetJumpSpeed))) "None" true)
        (if (>= (Variables|Default|GetJumpTime) 1.0)
          (CallFunction|ResetJump))))
    (:then_4
      (if (>= (Math|Vector|Distance(Vector) (Variables|Default|GetVelocity) _returnvalue_3) 1e+02)
        (if (Variables|Default|GetIsShaking)
          (Variables|Default|SetVelocity _returnvalue_3 :!label _label_3)
          (else
            (Variables|Default|SetIsShaking true)
            (Niagara|SetNiagaraVariable(Float) _decaldegeu "CustomEmission" 3e+01)
            (Utilities|FlowControl|Delay 0.2)
            (Niagara|SetNiagaraVariable(Float) _decaldegeu "CustomEmission" 0.0)
            (Variables|Default|SetVelocity _returnvalue_3)
            (Variables|Default|SetIsShaking false)
            (Camera|PlayWorldCameraShake "/Game/VFX/CSB_CameraShake.CSB_CameraShake_C" (Transformation|GetWorldLocation (Variables|Default|GetSkeletalMesh)) 1.0 2e+03 1.0 true)))
        (else
          (goto _label_3))))))

(event EventBeginPlay
  (bind _skeletalmesh (Variables|Default|GetSkeletalMesh))
  (bind _asbp_game_instance (Utilities|Casting|CastToBP_GameInstance (Game|GetGameInstance)))
  (Variables|Default|SetGameInstance _asbp_game_instance)
  (bind _returnvalue (Rendering|Material|CreateDynamicMaterialInstance _skeletalmesh 0 (Rendering|Material|GetMaterial _skeletalmesh 0) "None" :!class /Script/Engine.PrimitiveComponent))
  (Variables|Default|SetDynamicMaterialInstance _returnvalue)
  (Variables|Default|SetVelocity "0, 0, 0"))

(event EventDeath
  ;[1 1 1] Death/Restart
  (if (not (Variables|Default|GetImmune))
    (Camera|PlayWorldCameraShake "/Game/VFX/CSB_CameraShakeDeath.CSB_CameraShakeDeath_C" (Transformation|GetWorldLocation (Variables|Default|GetSkeletalMesh)) 1e+02 1e+06 1.0 true)
    (if (Variables|Default|GetHasHelmet)
      (Variables|Default|SetImmune true)
      (Rendering|SetVisibility (Variables|Default|GetHelmet) false false)
      (Variables|Default|SetHasHelmet false)
      (Utilities|FlowControl|Delay 1.0)
      (Variables|Default|SetImmune false)
      (else
        (Input|DisableInput (Game|GetPlayerController 0))
        (Variables|Default|SetImmune true)
        (CallFunction|DeathVFX)
        (Utilities|FlowControl|Delay 2.0)
        (CallFunction|ResetPlayer)))))

(event Input|ActionEvents|InputActionDash
  (params (Key :type Key%20Structure :default "None"))
  (bind _dashstrength (Variables|Default|GetDashStrength))
  (bind _skeletalmesh (Variables|Default|GetSkeletalMesh))
  (bind _skeletalmesh_2 (Variables|Default|GetSkeletalMesh))
  (bind _verticalsign (Variables|Default|GetVerticalSign))
  (bind _returnvalue (Transformation|GetComponentVelocity _skeletalmesh_2))
  (bind _returnvalue_2 (Transformation|GetWorldLocation _skeletalmesh))
  (bind _returnvalue_3 (< _verticalsign 0.0))
  (bind _returnvalue_4 (< (.z _returnvalue) 0.0))
  (bind _returnvalue_5 (and _returnvalue_4 _returnvalue_3))
  ;[1 1 1] Dash Function
  (:Pressed
    (if (Variables|Default|GetCanDash)
      (Utilities|FlowControl|Gate false :!label _label
        (:Exit
          (Utilities|FlowControl|Sequence
            (:then_0
              (Physics|SetEnableGravity (Variables|Default|GetSkeletalMesh) false)
              (Variables|Default|SetIsDashing true)
              (Variables|Default|SetCanDash false)
              (Variables|Default|SetDashEffectTimer 1.0)
              (if (> (Variables|Default|GetDashEffectTimer) 0.0) :!label _label_2
                (Class|PrimitiveComponent|SetAllPhysicsLinearVelocity _skeletalmesh_2 (Math|Vector|MakeVector 0.0 (.y _returnvalue) (Math|Float|SelectFloat (.z _returnvalue) (Math|Float|Lerp 0.0 (.z _returnvalue) (Variables|Default|GetDashEffectTimer)) _returnvalue_5)) false)
                (Variables|Default|SetDashEffectTimer (- (Variables|Default|GetDashEffectTimer) (* (Utilities|Time|GetWorldDeltaSeconds) 1e+01)))
                (Utilities|FlowControl|DelayUntilNextTick)
                (goto _label_2)
                (else
                  (Physics|AddImpulse _skeletalmesh_2 (Math|Vector|MakeVector 0.0 (* (stale Input|AxisEvents|InputAxisHorizontalAxis AxisValue) _dashstrength) (Math|Float|SelectFloat (* (* _dashstrength (stale Input|AxisEvents|InputAxisVerticalAxis AxisValue)) 2.0) (* _dashstrength (stale Input|AxisEvents|InputAxisVerticalAxis AxisValue)) _returnvalue_5)) "None" true)
                  (Utilities|FlowControl|Sequence
                    (:then_0
                      (Utilities|FlowControl|Delay 0.2)
                      (CallFunction|ResetDash))
                    (:then_1
                      (Niagara|SpawnSystematLocation 0 _returnvalue_2 (Math|Rotator|FindLookatRotation _returnvalue_2 (+ _returnvalue_2 (Transformation|GetComponentVelocity _skeletalmesh)))))))))
            (:then_1
              (goto _label Close))))))))

(event Input|ActionEvents|InputActionJump
  (params (Key :type Key%20Structure :default "None"))
  ;[1 1 1] Jump Functions
  (:Pressed
    (if (not (Variables|Default|GetIsJumping))
      (if (Variables|Default|GetCanJump)
        (if (not (Variables|Default|GetIsDashing))
          (Variables|Default|SetIsJumping true)))))
  (:Released
    (CallFunction|ResetJump)))

(event Input|AxisEvents|InputAxisHorizontalAxis
  (params (AxisValue :type Float%20%28single-precision%29))
  (bind _skeletalmesh (Variables|Default|GetSkeletalMesh))
  ;[1 1 1] Horizontal Movement
  (if (not (Variables|Default|GetIsDashing))
    (if (== AxisValue 0.0)
      (Variables|Default|SetRollCounterCurve (Math|Float|Clamp(Float) (- (Variables|Default|GetRollCounterCurve) (* (/ 1.0 (Variables|Default|GetDeccelerationTime)) (Utilities|Time|GetWorldDeltaSeconds)))))
      (Class|PrimitiveComponent|SetAllPhysicsLinearVelocity _skeletalmesh (Math|Vector|MakeVector 0.0 (* (Math|Curves|GetFloatValue (Variables|Default|GetWalkInCurve) (Variables|Default|GetRollCounterCurve)) (Variables|Default|GetHorizontalSpeed) (Variables|Default|GetHorizontalDirection)) (.z (Transformation|GetComponentVelocity _skeletalmesh))) false :!label _label)
      (else
        (Utilities|FlowControl|Sequence
          (:then_0
            (Variables|Default|SetRollCounterCurve (Math|Float|Clamp(Float) (+ (* (Math|Float|Absolute(Float) AxisValue) (/ 1.0 (Variables|Default|GetAccelerationTime))) (Variables|Default|GetRollCounterCurve))))
            (goto _label))
          (:then_1
            (if (> AxisValue 0.0)
              (Variables|Default|SetHorizontalDirection 1.0)
              (else
                (Variables|Default|SetHorizontalDirection -1.0)))))))))

(event Input|AxisEvents|InputAxisHorizontalAxis
  (params (AxisValue :type Float%20%28single-precision%29))
  ;[1 1 1] Dash Function
)

(event Input|AxisEvents|InputAxisVerticalAxis
  (params (AxisValue :type Float%20%28single-precision%29))
  ;[1 1 1] Vertical Movement
  (if (not (Variables|Default|GetIsDashing))
    (if (< AxisValue 0.0)
      (Variables|Default|SetVerticalSign -1.0)
      (Physics|AddForce (Variables|Default|GetSkeletalMesh) (Math|Vector|MakeVector 0.0 0.0 (* AxisValue (Variables|Default|GetVerticalSpeed))) "None" false)
      (else
        (Variables|Default|SetVerticalSign 1.0)))))

(fn ConstructionScript)