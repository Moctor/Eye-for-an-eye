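; Helmet pickup actor that grants a helmet to an overlapping actor implementing BP_PlayerInterface.
; The first valid Box overlap passes a DoOnce gate, calls EarnAHelmetMessage on that actor and starts the DestoryHelmet timeline.
; The timeline drives the helmet mesh's yaw and scale, then destroys the pickup when finished.
; A relative-height update from the timeline's Pos track exists but is disconnected and never runs.
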(event OnComponentBeginOverlap(Box)
  (params (OverlappedComponent :type Primitive%20Component%20Object%20Reference) (OtherActor :type Actor%20Object%20Reference) (OtherComp :type Primitive%20Component%20Object%20Reference) (OtherBodyIndex :type Integer) (bFromSweep :type Boolean) (SweepResult :type Hit%20Result%20Structure%20%28by%20ref%29))
  (bind _helmet (Variables|Default|GetHelmet))
  (if (Utilities|DoesObjectImplementInterface OtherActor "/Game/Blueprint/Player/BP_PlayerInterface.BP_PlayerInterface_C")
    (Utilities|FlowControl|DoOnce false
      (:Completed
        (Class|BPPlayerInterface|EarnAHelmet(Message) OtherActor)
        (bind (_direction _pos _rot _scale) (Timeline|DestoryHelmet PlayFromStart)
          (:Update
            (Transformation|SetWorldRotation _helmet (Math|Rotator|MakeRotator 0.0 0.0 _rot) false false)
            (Transformation|SetRelativeScale3D _helmet (Math|Conversions|ToVector(Float) _scale)))
          (:Finished
            (Actor|DestroyActor)))))))

(fn ConstructionScript)